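; Breakable target actor that swaps its static mesh for a fractured statue Geometry Collection when damaged hard enough.
; Hits apply self-damage equal to the normal impulse magnitude, feeding the any-damage handler.
; Damage above the collection's first threshold assigns the statue collection, applies strain at the last hit location plus a radial impulse, and disables the mesh.
; Chaos break events switch broken pieces to the Debris collision profile.
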(event `self.ReceiveBeginPlay`
  (add `self.OnTakeAnyDamage` (delegate `CustomEvent`)))

(event `CustomEvent` :!signature `self.OnTakeAnyDamage`
  (params (DamagedActor :type "Actor Object Reference") (Damage :type "Float (single-precision)") (DamageType :type "DamageType Object Reference") (InstigatedBy :type "Controller Object Reference") (DamageCauser :type "Actor Object Reference"))
  (bind _staticmesh (`self.StaticMesh`))
  (if (> Damage (`|GetArrayItem` (`GeometryCollectionComponent.DamageThreshold` (`self.GeometryCollection`))))
    (`GeometryCollectionComponent.SetRestCollection` (`self.GeometryCollection`) "/Game/StarterContent/Props/SM_Statue_SM_Statue/GC_SM_Statue.GC_SM_Statue" false)
    (`GeometryCollectionComponent.ApplyExternalStrain` (`self.GeometryCollection`) 0 (stale `self.ReceiveHit` HitLocation) 100.0 0 1.0 10000000.0)
    (`PhysicsObjectBlueprintLibrary.ApplyRadialImpulse` null (`self.K2_GetActorLocation`) 100.0 200.0 "RIF_Constant")
    (`SceneComponent.SetVisibility` (`self.StaticMesh`) false false)
    (`PrimitiveComponent.SetSimulatePhysics` _staticmesh false)
    (`PrimitiveComponent.SetCollisionEnabled` _staticmesh "NoCollision")
    (`PrimitiveComponent.SetWalkableSlopeOverride` (`self.GeometryCollection`) (make `WalkableSlopeOverride` "WalkableSlope_Unwalkable"))))

(event `self.ReceiveHit`
  (params (MyComp :type "PrimitiveComponent Object Reference") (Other :type "Actor Object Reference") (OtherComp :type "PrimitiveComponent Object Reference") (bSelfMoved :type Boolean) (HitLocation :type "Vector Structure") (HitNormal :type "Vector Structure") (NormalImpulse :type "Vector Structure") (Hit :type "HitResult Structure (by ref)"))
  (`GameplayStatics.ApplyDamage` self (`KismetMathLibrary.VSize` NormalImpulse)))

(event `self.GeometryCollection.OnChaosBreakEvent`
  (params (BreakEvent :type "ChaosBreakEvent Structure (by ref)"))
  (`GeometryCollectionComponent.SetPerParticleCollisionProfileName` (`self.GeometryCollection`) (`|MakeArray` BreakEvent_Index) "Debris"))

(fn `UserConstructionScript`)